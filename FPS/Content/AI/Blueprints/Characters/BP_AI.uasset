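; BP_AI is an AI character that takes hits, tracks life and shows it on a world-space life bar.
; Each hit deals fixed damage, updates the WB_AI_LifeBar widget with normalized life and checks for death.
; Blackboard booleans signal hit, attack and death states, presumably for a behavior tree.
; Tick turns the life bar toward the player, while LookAtPlayer rotates the mesh toward them with a height offset.
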(event `self.ReceiveBeginPlay`
  (set `self.AIControllerClass` (`self.AI Controller Class`))
  (set `self.Life` (`self.MaxLife`)))

(event `self.ReceiveTick`
  (params (DeltaSeconds :type "Float (single-precision)"))
  (`SceneComponent.K2_SetWorldRotation` (`self.W_LifeBar`) (`KismetMathLibrary.FindLookAtRotation` (`SceneComponent.K2_GetComponentLocation` (`self.W_LifeBar`)) (`self.K2_GetActorLocation` (`/Game/FL_Utils.GetMyPlayer`))) false false))

(event `/Game/Weapons/I_Hitteable.Hit`
  (params (Damage :type "Float (double-precision)") (HitComponent :type "PrimitiveComponent Object Reference"))
  (`self.GetHit` 10.0)
  (`self.UpdateLife` 10.0)
  (`self.CheckIfDead`))

(fn `AttackBehavior`
  (`BlackboardComponent.SetValueAsBool` (`AIBlueprintHelperLibrary.GetBlackboard` null) "isAttacking" true))

(fn `CheckIfDead`
  (if (<= (`self.Life`) 0.0)
    (`BlackboardComponent.SetValueAsBool` (`AIBlueprintHelperLibrary.GetBlackboard` null) "isDead" true)))

(fn `GetHit`
  (params (Damage :type "Float (double-precision)"))
  (`BlackboardComponent.SetValueAsBool` (`AIBlueprintHelperLibrary.GetBlackboard` null) "isHit" true)
  (`KismetSystemLibrary.PrintString` "Hit"))

(fn `LookAtPlayer`
  (params (MeshInitRot :type "Rotator Structure"))
  (bind (_returnvalue_x _returnvalue_y _returnvalue_z) (`KismetMathLibrary.BreakVector` (`self.K2_GetActorLocation` (`/Game/FL_Utils.GetMyPlayer`))))
  (`SceneComponent.K2_SetRelativeRotation` (`self.Mesh`) (`KismetMathLibrary.ComposeRotators` MeshInitRot (`KismetMathLibrary.FindLookAtRotation` (`SceneComponent.K2_GetComponentLocation` (`self.Mesh`)) (`KismetMathLibrary.MakeVector` _returnvalue_x _returnvalue_y (- _returnvalue_z 80.0)))) false false))

(fn `UpdateLife`
  (params (Damage :type "Float (double-precision)"))
  (set `self.Life` (- (`self.Life`) Damage))
  (`self.UpdateWidget` (`KismetMathLibrary.NormalizeToRange` (`self.Life`) 0.0 (`self.MaxLife`))))

(fn `UpdateWidget`
  (params (InPercent :type "Float (single-precision)"))
  (bind _aswb_ai_life_bar (cast `/Game/AI/WB_AI_LifeBar` (`WidgetComponent.GetWidget` (`self.W_LifeBar`))))
  (`/Game/AI/WB_AI_LifeBar.UpdateLifeBar` _aswb_ai_life_bar InPercent))

(fn `UserConstructionScript`)