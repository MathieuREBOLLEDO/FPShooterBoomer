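; BP_AI_Flying is a flying AI character that faces the player and attacks with projectiles.
; On BeginPlay it switches character movement to Flying and caches the mesh's initial relative transform.
; Each tick it runs the parent logic, then calls LookAtPlayer with the cached mesh rotation.
; Its AttackBehavior event spawns a BP_Projectile at the Muzzle's world location and rotation.
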(event `self.ReceiveBeginPlay`
  (`parent.ReceiveBeginPlay`)
  (`CharacterMovementComponent.SetMovementMode` (`self.CharacterMovement`) "MOVE_Flying" 0)
  (set `self.MeshInitLocation` (`SceneComponent.RelativeLocation` (`self.Mesh`)))
  (set `self.MeshInit Rotation` (`SceneComponent.RelativeRotation` (`self.Mesh`))))

(event `self.ReceiveTick`
  (params (DeltaSeconds :type "Float (single-precision)"))
  (`parent.ReceiveTick` DeltaSeconds)
  (`self.LookAtPlayer` (`self.MeshInit Rotation`)))

(event `self.AttackBehavior`
  (`|SpawnActorFromClass` "/Game/AI/BP_Projectile.BP_Projectile_C" (`KismetMathLibrary.MakeTransform` (`SceneComponent.K2_GetComponentLocation` (`self.Muzzle`)) (`SceneComponent.K2_GetComponentRotation` (`self.Muzzle`))) "Undefined" "MultiplyWithRoot" null 5.0 null))

(fn `UserConstructionScript`
  (`parent.UserConstructionScript`))