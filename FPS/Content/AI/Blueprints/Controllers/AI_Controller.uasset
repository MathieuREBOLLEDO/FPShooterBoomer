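; AI controller Blueprint that switches behavior trees based on an AI state enum.
; BeginPlay runs the current behavior tree, and OnstateChange stores the new state and runs the tree mapped to it in MapOfState.
; Tick prints the current state to screen every frame.
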(event `self.ReceiveBeginPlay`
  (`self.RunBehaviorTree` (`self.CurrentBehaviorTree`)))

(event `self.ReceiveTick`
  (params (DeltaSeconds :type "Float (single-precision)"))
  (`KismetSystemLibrary.PrintString` (`|GetEnumeratorNameAsString` (`self.CurrentState`))))

(fn `OnstateChange`
  (params (NewState :type "/Game/AI/E_AI_States Enum" :default "NewEnumerator0"))
  (set `self.CurrentState` NewState)
  (`self.RunBehaviorTree` (`BlueprintMapLibrary.Map_Find` (`self.MapOfState`) NewState)))

(fn `UserConstructionScript`)