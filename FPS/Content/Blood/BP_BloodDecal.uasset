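; BP_BloodDecal is a blood decal actor that acts as a health pickup for the player.
; On BeginPlay it places the decal using its Location and Rotation variables, and DecalSize sets both the decal scale and the trigger box extent.
; When a BP_Player overlaps the box, it calls the player's CallHealedPlayer with a fixed amount and destroys itself.
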(event `self.ReceiveBeginPlay`
  (`BoxComponent.SetBoxExtent` (`self.Box`) (`KismetMathLibrary.Conv_DoubleToVector` (`self.decalSize`)) true)
  (`SceneComponent.K2_SetWorldLocation` (`self.Decal`) (`self.Location`) false false)
  (`SceneComponent.K2_SetWorldRotation` (`self.Decal`) (`self.Rotation`) false false)
  (`SceneComponent.SetRelativeScale3D` (`self.Decal`) (`KismetMathLibrary.Conv_DoubleToVector` (`self.decalSize`))))

(event `self.Box.OnComponentBeginOverlap`
  (params (OverlappedComponent :type "PrimitiveComponent Object Reference") (OtherActor :type "Actor Object Reference") (OtherComp :type "PrimitiveComponent Object Reference") (OtherBodyIndex :type Integer) (bFromSweep :type Boolean) (SweepResult :type "HitResult Structure (by ref)"))
  (bind _asbp_player (cast `/Game/Player/Blueprints/BP_Player` OtherActor))
  (`/Game/Player/Blueprints/BP_Player.HealedPlayer` _asbp_player 5.0)
  (`self.K2_DestroyActor`))

(fn `UserConstructionScript`)