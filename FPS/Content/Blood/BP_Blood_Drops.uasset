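; BP_Blood_Drops is a blood effect actor that leaves decals where its Niagara particles report data.
; On BeginPlay it passes itself to the Niagara system as the BP_Blood variable, so particle data is exported back to it.
; For each exported particle, it spawns a blood decal at that position, rotated to face against the particle's velocity.
; Unconnected nodes for spawning BP_BloodDecal and fading it out never run.
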(event `self.ReceiveBeginPlay`
  (`NiagaraComponent.SetVariableObject` (`self.NS_Blood_Effect`) "BP_Blood" self))

(event `self.ReceiveParticleData`
  (params (Data :type "Array of BasicParticleData Structure (by ref)") (NiagaraSystem :type "NiagaraSystem Object Reference") (SimulationPositionOffset :type "Vector Structure (by ref)"))
  (for _array_element Data
    (bind (_position _size _velocity) (break `BasicParticleData` _array_element))
    (`GameplayStatics.SpawnDecalAtLocation` "/Game/Blood/M_Blood_Decal_Inst.M_Blood_Decal_Inst" (`KismetMathLibrary.Conv_DoubleToVector` (`self.DecalSize`)) _position (`KismetMathLibrary.Conv_VectorToRotator` (* _velocity -1.0)))))

(fn `UserConstructionScript`)