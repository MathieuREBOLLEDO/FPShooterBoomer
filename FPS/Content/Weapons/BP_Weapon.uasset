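; Weapon actor that adds its input mapping context on begin play and handles the player's shoot and melee inputs, gated by a state enum.
; Shooting flashes a point light, spawns Niagara effects at the muzzle and sphere-traces from the first-person camera, sending damage through I_Hitteable to every implementing hit actor.
; Melee only changes state, and nothing here resets the state afterward.
; It also caches the player's state and provides a relative-transform lerp helper.
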(event `self.ReceiveBeginPlay`
  (bind _returnvalue (pcsubsystem `EnhancedInputLocalPlayerSubsystem` (`GameplayStatics.GetPlayerController` 0)))
  (`/Engine/EditorBlueprintResources/StandardMacros.IsValid` _returnvalue
    (:`Is Valid`
      (`EnhancedInputSubsystemInterface.AddMappingContext` _returnvalue "/Game/Player/Input/IMC_Weapons.IMC_Weapons" 1 (struct))
      (set `self.currentState` "NewEnumerator0")
      (add `/Game/Player/Blueprints/BP_Player.ChangedState` (`/Game/FL_Utils.GetMyPlayer`) (delegate `UpdateStateMeca`)))))

(event `UpdateStateMeca`
  (params (playerStateMeca :type "/Game/E_StateMeca Enum" :default "NewEnumerator0"))
  (set `self.playerStateMeca` playerStateMeca))

(event `EnhancedInput|/Game/Player/Input/Actions/IA_Shoot`
  (params (ActionValue :type Boolean) (ElapsedSeconds :type "Float (double-precision)") (TriggeredSeconds :type "Float (double-precision)") (InputAction :type "InputAction Object Reference" :default "/Game/Player/Input/Actions/IA_Shoot.IA_Shoot"))
  (:`Triggered`
    (if (`|EnumEquality` (`self.currentState`) "NewEnumerator0")
      (`self.ShootFunction`))))

(event `EnhancedInput|/Game/Player/Input/Actions/IA_Melee`
  (params (ActionValue :type Boolean) (ElapsedSeconds :type "Float (double-precision)") (TriggeredSeconds :type "Float (double-precision)") (InputAction :type "InputAction Object Reference" :default "/Game/Player/Input/Actions/IA_Melee.IA_Melee"))
  (:`Triggered`
    (if (`|EnumEquality` (`self.currentState`) "NewEnumerator0")
      (`self.MeleeFunction`))))

(fn `MeleeFunction`
  (set `self.currentState` "NewEnumerator3"))

(fn `NewFunction`)

(fn `PlayFeedBackAtMuzzleLocation`
  (params (`Niagara Systems` :type "Array of NiagaraSystem Object Reference"))
  (bind _muzzle (`self.Muzzle`))
  (for _array_element `Niagara Systems`
    (`NiagaraFunctionLibrary.SpawnSystemAtLocation` _array_element (`SceneComponent.K2_GetComponentLocation` _muzzle) (`SceneComponent.K2_GetComponentRotation` _muzzle))))

(fn `SetRelativeRotAndLoc`
  (params (RotationToGo :type "Rotator Structure") (AlphaRotation :type "Float (single-precision)") (LocationToGo :type "Vector Structure") (AlphaLocation :type "Float (single-precision)"))
  (`self.K2_SetActorRelativeRotation` (`KismetMathLibrary.RLerp` (struct) RotationToGo AlphaRotation))
  (`self.K2_SetActorRelativeLocation` (`KismetMathLibrary.VLerp` (0.0 0.0 0.0) LocationToGo AlphaLocation)))

(fn `ShootFunction`
  (`SceneComponent.SetVisibility` (`self.PointLight`) true false)
  (set `self.currentState` "NewEnumerator1")
  (`self.PlayFeedBackAtMuzzleLocation` (`self.FeedBackAtMuzzle`))
  (`self.ShootTrace`)
  (`SceneComponent.SetVisibility` (`self.PointLight`) false false))

(fn `ShootTrace`
  (bind _firstpersoncamera (`/Game/Player/Blueprints/BP_Player.FirstPersonCamera` (`/Game/FL_Utils.GetMyPlayer`)))
  (bind _returnvalue (`SceneComponent.K2_GetComponentLocation` _firstpersoncamera))
  (bind _outhits (`KismetSystemLibrary.SphereTraceMulti` _returnvalue (+ _returnvalue (* (`SceneComponent.GetForwardVector` _firstpersoncamera) (`self.WeaponRange`))) (`self.WeaponSpread`) "TraceTypeQuery1" false (`|MakeArray` (`/Game/FL_Utils.GetMyPlayer`) :!type "Actor Object Reference")))
  (for _array_element _outhits
    (bind (_bblockinghit _binitialoverlap _time _distance _location _impactpoint _normal _impactnormal _physmat _hitactor _hitcomponent) (`GameplayStatics.BreakHitResult` _array_element))
    (if (`KismetSystemLibrary.DoesImplementInterface` _hitactor "/Game/Weapons/I_Hitteable.I_Hitteable_C")
      (message `/Game/Weapons/I_Hitteable.Hit` _hitactor (`self.WeaponDamage`) _hitcomponent _location _normal "NewEnumerator2"))))

(fn `UserConstructionScript`)