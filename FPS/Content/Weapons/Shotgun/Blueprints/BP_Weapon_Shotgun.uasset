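; Shotgun weapon Blueprint that adds procedural animation, sound and shell ejection to its parent's main shot, special shot, melee and reload.
; Timelines drive relative transforms for recoil, reload turn and melee motion instead of skeletal animations.
; Both shots share the recoil, which on finish hides the point light, chains into the reload motion and spawns an empty shell after a short timer.
; Timeline completions update the weapon's CurrentState.
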(event `ThrowShellAnim`
  ;[1 1 1] ThrowShellAnim
  (`KismetSystemLibrary.K2_SetTimerDelegate` (delegate `SpawnShell`) 0.3))

(event `SpawnShell`
  ;[1 1 1] ThrowShellAnim
  (`|SpawnActorFromClass` "/Game/Weapons/Shotgun/Blueprints/BP_EmptyShell.BP_EmptyShell_C" (`KismetMathLibrary.MakeTransform` (`SceneComponent.K2_GetComponentLocation` (`self.Mesh`)) (struct) (2.3 2.3 2.3)) "Undefined" "MultiplyWithRoot" null null))

(event `PlayShoot`
  ;[1 1 1] Shoot Anim Part
  (bind (_direction _back _roll) (`Timeline|ShootTimeline` :!via `PlayFromStart`)
    (:`Update`
      (`self.SetRelativeRotAndLoc` (`self.PushTurn`) _back (`self.PushBack`) _roll))
    (:`Finished`
      (`SceneComponent.SetVisibility` (`self.PointLight`) false false)
      (`GameplayStatics.PlaySound2D` "/Game/Weapons/Shotgun/SFX/P_Shotgun_Reload.P_Shotgun_Reload" 1.0 1.0 0.0 null null)
      (`|ExecutionSequence`
        (:`then_0`
          (`self.ThrowShellAnim`))
        (:`then_1`
          (`self.PlayReload`)
          (set `self.currentState` "NewEnumerator2"))))))

(event `self.mainShootFunction`
  (`parent.mainShootFunction`)
  (`self.PlayShoot`)
  (`GameplayStatics.PlaySound2D` "/Game/Weapons/Shotgun/SFX/P_Shotgun_Shoot.P_Shotgun_Shoot" 1.0 1.0 0.0 null null))

(event `ReloadAnim`
  (`self.ThrowShellAnim`)
  (`GameplayStatics.PlaySound2D` "/Game/Weapons/Shotgun/SFX/P_DoubleShotgun_Reload.P_DoubleShotgun_Reload" 1.0 1.0 0.0 null null)
  (`self.PlayReload`))

(event `PlayReload`
  ;[1 1 1] Reload Animatiom part
  (bind (_direction _reload) (`Timeline|ReloadTimeline` :!via `PlayFromStart`)
    (:`Update`
      (`self.K2_SetActorRelativeRotation` (`KismetMathLibrary.RLerp` (struct) (`self.ReloadRotation`) _reload)))
    (:`Finished`
      (set `self.currentState` "NewEnumerator0"))))

(event `self.MeleeFunction`
  (`parent.MeleeFunction`)
  (`self.PlayMelee`))

(event `self.SpecialShoot Function`
  (`parent.specialShoot Function`)
  (`self.PlayShoot`)
  (`GameplayStatics.PlaySound2D` "/Game/Weapons/Shotgun/SFX/P_Shotgun_Shoot.P_Shotgun_Shoot" 1.0 1.0 0.0 null null))

(event `PlayMelee`
  ;[1 1 1] Melee Anim part
  (bind (_direction _meleerotation _meleeforward) (`Timeline|MeleeTimeline` :!via `PlayFromStart`)
    (:`Update`
      (`self.SetRelativeRotAndLoc` (`self.MeeleRotation`) _meleerotation (`self.MeleeForward`) _meleeforward))
    (:`Finished`
      (set `self.currentState` "NewEnumerator0"))))

(fn `UserConstructionScript`
  (`parent.UserConstructionScript`))